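; UDP listener that receives finger sensor data over the network and forwards it to the SensorController.
; It opens the receive socket on BeginPlay, closes it on EndPlay, and parses each incoming packet as a JSON string.
; For "fingerData" messages it resolves the sensor name to an enum, then passes the five finger values to DataReceive as floats, printing a message for unknown sensors.
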(event `self.ReceiveBeginPlay`
  (bind _udp (`self.UDP`))
  (`UDPComponent.StartReceiveSocketListening` _udp 7755)
  (add `UDPComponent.OnReceivedBytes` _udp (delegate `UDPReceivedEvent`)))

(event `self.ReceiveEndPlay`
  (params (EndPlayReason :type "EEndPlayReason Enum" :default "Destroyed"))
  (`UDPComponent.CloseReceiveSocket` (`self.UDP`)))

(event `UDPReceivedEvent`
  (params (Bytes :type "Array of Byte (by ref)"))
  (bind _returnvalue (`UDPComponent.StringFromBinaryArray` (`self.UDP`) Bytes))
  (bind _returnvalue_2 (`SIOJsonValue.AsObject` (`SIOJsonValue.ValueFromJsonString` _returnvalue)))
  (if (`KismetStringLibrary.EqualEqual_StrStr` (`SIOJsonObject.GetStringField` _returnvalue_2 "type") "fingerData")
    (bind _returnvalue_3 (`SIOJsonObject.GetStringField` _returnvalue_2 "sensorName"))
    (bind _gyrosensor (`/Game/Blueprints/FingerController.GetSensorBoneEnumFromString` (`self.SensorController`) _returnvalue_3))
    (if (`|EnumEquality` _gyrosensor "NewEnumerator0")
      (`KismetSystemLibrary.PrintString` (`KismetStringLibrary.Concat_StrStr` "Sensor " _returnvalue_3 " not found"))
      (else
        (`|ExecutionSequence`
          (:`then_0`
            (`/Game/Blueprints/FingerController.DataReceive` (`self.SensorController`) _gyrosensor "NewEnumerator5" (`KismetStringLibrary.Conv_StringToDouble` (`SIOJsonObject.GetStringField` _returnvalue_2 "Thumb"))))
          (:`then_1`
            (`/Game/Blueprints/FingerController.DataReceive` (`self.SensorController`) _gyrosensor "NewEnumerator6" (`KismetStringLibrary.Conv_StringToDouble` (`SIOJsonObject.GetStringField` _returnvalue_2 "Index"))))
          (:`then_2`
            (`/Game/Blueprints/FingerController.DataReceive` (`self.SensorController`) _gyrosensor "NewEnumerator7" (`KismetStringLibrary.Conv_StringToDouble` (`SIOJsonObject.GetStringField` _returnvalue_2 "Middle"))))
          (:`then_3`
            (`/Game/Blueprints/FingerController.DataReceive` (`self.SensorController`) _gyrosensor "NewEnumerator14" (`KismetStringLibrary.Conv_StringToDouble` (`SIOJsonObject.GetStringField` _returnvalue_2 "Ring"))))
          (:`then_4`
            (`/Game/Blueprints/FingerController.DataReceive` (`self.SensorController`) _gyrosensor "NewEnumerator15" (`KismetStringLibrary.Conv_StringToDouble` (`SIOJsonObject.GetStringField` _returnvalue_2 "Pinky")))))))))

(fn `UserConstructionScript`)