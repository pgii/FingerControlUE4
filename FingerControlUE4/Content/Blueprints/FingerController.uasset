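; Finger controller that drives a character's finger bones from incoming sensor values.
; DataReceive looks up the matching sensor and bone entry in FingerBoneStructArray and ignores unmatched pairs.
; It remaps the value through that entry's ranges with a clamped linear map that assumes InMin exceeds InMax.
; The result goes to TPoseCharacter's Mixamo finger-control Anim Blueprint with smoothing parameters.
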(event `DataReceive`
  (params (fingerSensorEnum :type "/Game/Blueprints/FingerSensorEnum Enum" :default "NewEnumerator0") (fingerBoneEnum :type "/Game/Blueprints/FingerBoneEnum Enum" :default "NewEnumerator0") (value :type "Float (double-precision)"))
  ;[1 0 0.5519] Data Receive
  (`self.UpdateFingerAnimClass` fingerSensorEnum fingerBoneEnum value))

(fn `GetFingerBoneStructFromFingerSensor`
  (params (fingerSensorEnum :type "/Game/Blueprints/FingerSensorEnum Enum" :default "NewEnumerator0") (fingerBoneEnum :type "/Game/Blueprints/FingerBoneEnum Enum" :default "NewEnumerator0"))
  (returns (SkeletonBoneStruct :type "/Game/Blueprints/FingerBoneStruct Structure") (isFound :type Boolean))
  (for _array_element (`self.FingerBoneStructArray`)
    (bind (_fingersensor _fingerbone) (break `/Game/Blueprints/FingerBoneStruct` _array_element))
    (if (and (`|EnumEquality` _fingersensor fingerSensorEnum) (`|EnumEquality` _fingerbone fingerBoneEnum))
      (return _array_element true)))
  (return (make `/Game/Blueprints/FingerBoneStruct` "NewEnumerator0") false))

(fn `GetSensorBoneEnumFromString`
  (params (GyroSensorString :type String))
  (returns (GyroSensor :type "/Game/Blueprints/FingerSensorEnum Enum"))
  (bind _enumvalue (foreach `/Game/Blueprints/FingerSensorEnum` false)
    (:`LoopBody`
      (if (`KismetStringLibrary.EqualEqual_StrStr` (`|GetEnumeratorNameAsString` _enumvalue) GyroSensorString)
        (return _enumvalue)))
    (:`then`
      (return "NewEnumerator0"))))

(fn `MapFingerValue`
  (params (value :type "Float (double-precision)") (inMin :type "Float (double-precision)") (inMax :type "Float (double-precision)") (outMin :type "Float (double-precision)") (outMax :type "Float (double-precision)" :default 0.0))
  (returns (result :type "Float (double-precision)"))
  (if (< inMin value)
    (return outMin)
    (elif (> value inMax)
      (return (+ (/ (* (- value inMin) (- outMax outMin)) (- inMax inMin)) outMin))
      (else
        (return outMax)))))

(fn `UpdateFingerAnimClass`
  (params (fingerSensorEnum :type "/Game/Blueprints/FingerSensorEnum Enum" :default "NewEnumerator0") (fingerBoneEnum :type "/Game/Blueprints/FingerBoneEnum Enum" :default "NewEnumerator0") (value :type "Float (double-precision)"))
  (bind (_skeletonbonestruct _isfound) (`self.GetFingerBoneStructFromFingerSensor` fingerSensorEnum fingerBoneEnum))
  (if _isfound
    (bind _asmixamo_finger_control_anim_bp (cast `/Game/MixamoCharacter/Mixamo_FingerControl_Anim_BP` (`SkeletalMeshComponent.GetAnimInstance` (`Character.Mesh` (`self.TPoseCharacter`)))))
    (bind (_fingersensor _fingerbone _inminmax _outminmax) (break `/Game/Blueprints/FingerBoneStruct` _skeletonbonestruct))
    (bind (_x _y) (`KismetMathLibrary.BreakVector2D` _inminmax))
    (bind (_x_2 _y_2) (`KismetMathLibrary.BreakVector2D` _outminmax))
    (bind _result (`self.MapFingerValue` value _x _y _x_2 _y_2))
    (`/Game/MixamoCharacter/Mixamo_FingerControl_Anim_BP.FingerDataReceive` _asmixamo_finger_control_anim_bp _fingersensor _fingerbone _result (`self.SmoothDeltaTime`) (`self.SmoothInterpSpeed`))
    (return)
    (else
      (return))))

(fn `UserConstructionScript`)